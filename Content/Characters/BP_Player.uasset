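; BP_Player is the player character Blueprint, handling movement and mouse-look input.
; Forward/Backward and Right/Left axis events add movement input along the actor's own forward and right vectors.
; Yaw and pitch look axes each pass through a gate that opens only while the right mouse button is held.
; The same button hides the cursor on press and shows it again on release.
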(event `InputAxis|Forward/Backward`
  (params (AxisValue :type "Float (single-precision)"))
  ;[1 1 1] Forward/Backward Right/Left WASD
  (`self.AddMovementInput` (`self.GetActorForwardVector`) AxisValue))

(event `InputAxis|Right/Left`
  (params (AxisValue :type "Float (single-precision)"))
  ;[1 1 1] Forward/Backward Right/Left WASD
  (`self.AddMovementInput` (`self.GetActorRightVector`) AxisValue))

(event `InputAxis|Look Right/Left`
  (params (AxisValue :type "Float (single-precision)"))
  ;[1 1 1] Look Up/Down Left/Right Mouse
  (`/Engine/EditorBlueprintResources/StandardMacros.Gate` true :!label _label
    (:`Exit`
      (`self.AddControllerYawInput` AxisValue))))

(event `Key|RightMouseButton`
  (params (Key :type "Key Structure"))
  (bind _returnvalue (`GameplayStatics.GetPlayerController` 0))
  ;[1 1 1] Look Up/Down Left/Right Mouse
  (:`Pressed`
    (set `PlayerController.bShowMouseCursor` false _returnvalue)
    (goto _label :!via `Open`))
  (:`Released`
    (set `PlayerController.bShowMouseCursor` true _returnvalue)
    (goto _label :!via `Close`)))

(event `InputAxis|Look Up/Down`
  (params (AxisValue :type "Float (single-precision)"))
  ;[1 1 1] Look Up/Down Left/Right Mouse
  (`/Engine/EditorBlueprintResources/StandardMacros.Gate` true :!label _label_2
    (:`Exit`
      (`self.AddControllerPitchInput` AxisValue))))

(event `Key|RightMouseButton`
  (params (Key :type "Key Structure"))
  (bind _returnvalue (`GameplayStatics.GetPlayerController` 0))
  ;[1 1 1] Look Up/Down Left/Right Mouse
  (:`Pressed`
    (set `PlayerController.bShowMouseCursor` false _returnvalue)
    (goto _label_2 :!via `Open`))
  (:`Released`
    (set `PlayerController.bShowMouseCursor` true _returnvalue)
    (goto _label_2 :!via `Close`)))

(fn `UserConstructionScript`)